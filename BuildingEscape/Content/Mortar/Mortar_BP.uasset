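; Mortar_BP is a player-controlled mortar with a Dome turret, a Barrel and an orbiting camera.
; On BeginPlay it hands the Barrel and Dome to its MortarAiming component.
; Azimuth input yaws the AzimuthGimbal and elevation input pitches the SpringArm, so the axes rotate on separate components.
; The Fire action delegates to MortarAiming.
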(event EventBeginPlay
  ;[1 1 1] Initialise Mortar Aiming Component
  (Class|AimingComponent|Initialise (Variables|Default|GetMortarAiming) (Variables|Default|GetBarrel) (Variables|Default|GetDome)))

(event Input|ActionEvents|InputActionFire
  (params (Key :type Key%20Structure))
  ;[1 1 1] Fire Input Binding
  (:Pressed
    (Class|AimingComponent|Fire (Variables|Default|GetMortarAiming))))

(event Input|AxisEvents|InputAxisAimAzimuth
  (params (AxisValue :type Float%20%28single-precision%29))
  ;[1 1 1] Camera Input Binding
  (Transformation|AddLocalRotation (Variables|Default|GetAzimuth%20Gimbal) (Math|Rotator|MakeRotator 0.0 0.0 AxisValue) false false))

(event Input|AxisEvents|InputAxisAimElevation
  (params (AxisValue :type Float%20%28single-precision%29))
  ;[1 1 1] Camera Input Binding
  (Transformation|AddLocalRotation (Variables|Default|GetSpringArm) (Math|Rotator|MakeRotator 0.0 AxisValue 0.0) false false))

(fn ConstructionScript)